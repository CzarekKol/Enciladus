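; Melee attack component that sphere-traces along sockets, damaging actors with the enemy tag and launching Characters for knockback.
; The 2D mode runs on Tick, chaining multi-traces through sprite sockets until a delay ends the attack.
; The 3D modes use looping timers to trace at one skeletal mesh socket or between two, until StopAttack clears the timer.
; An ignore list prevents repeat hits within a swing.
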(event Custom|Melee%20trace%20attack%202D
  (params (Sprite :type Paper%20Flipbook%20Component%20Object%20Reference) (Damage :type Float%20%28double-precision%29) (Attack%20Duration :type Float%20%28double-precision%29) (Attack%20Radius :type Float%20%28double-precision%29) (Knockback%20Force :type Vector) (Enemy%20Tag%20Container :type Name) (IsAttaclomg :type Boolean) (Socket%20Array :type Array%20of%20Names))
  ;[1 1 1] Add Variables
  (Variables|Default|SetSprite Sprite)
  (Variables|Default|SetDamage Damage)
  (Variables|Default|SetAttack%20Duration Attack%20Duration)
  (Variables|Default|SetAttack%20Radius Attack%20Radius)
  (Variables|Default|SetKnockback%20Force Knockback%20Force)
  (Variables|Default|SetEnemy%20Tag%20Container Enemy%20Tag%20Container)
  (Variables|Default|SetIs%20Attaclomg IsAttaclomg)
  (Variables|Default|SetSocket%20Array Socket%20Array))

(event Custom|Mele%20Trace%20Attack%203D%20for%20one%20socket
  (params (SocketName :type Name) (Enemy%20Tag%20Container :type Name) (Damage :type Float%20%28double-precision%29) (Attack%20Radius :type Float%20%28double-precision%29) (KnockbackForce :type Vector) (Skeleton%20Mesh :type Skeletal%20Mesh%20Component%20Object%20Reference))
  ;[1 1 1] Mele Attack Calculation for 3D model with one socket attached
  (Variables|Default|SetSocket%20Name SocketName)
  (Variables|Default|SetEnemy%20Tag%20Container Enemy%20Tag%20Container)
  (Variables|Default|SetDamage Damage)
  (Variables|Default|SetAttack%20Radius Attack%20Radius)
  (Variables|Default|SetKnockback%20Force KnockbackForce)
  (Variables|Default|SetSkeleton%20Mesh%20Reference Skeleton%20Mesh)
  (CallFunction|TriggerAttackOneSocket))

(event Custom|StartAtack2
  (bind _socket_array (Variables|Default|GetSocket%20Array))
  ;[1 1 1] Melle Attack Calculation for 3D models with exact 2 sockets
  (bind _outhit (Collision|SphereTraceByChannel (Transformation|GetSocketLocation (Variables|Default|GetSkeleton%20Mesh%20Reference) (Utilities|Array|Get(acopy) _socket_array)) (Transformation|GetSocketLocation (Variables|Default|GetSkeleton%20Mesh%20Reference) (Utilities|Array|Get(acopy) _socket_array 1)) (Variables|Default|GetAttack%20Radius) "TraceTypeQuery2" false (Variables|Default|GetActors%20to%20Ignore) "ForOneFrame"))
  (Utilities|Array|Add (Variables|Default|GetActors%20to%20Ignore) (.HitActor (Collision|BreakHitResult _outhit)))
  (Utilities|IsValid (.HitActor (Collision|BreakHitResult _outhit))
    (:Is%20Valid
      (if (Utilities|Array|ContainsItem (Variables|/Script/Engine.Actor|GetTags (.HitActor (Collision|BreakHitResult _outhit))) (Variables|Default|GetEnemy%20Tag%20Container))
        (Game|Damage|ApplyDamage (.HitActor (Collision|BreakHitResult _outhit)) (Variables|Default|GetDamage) 0 0)
        (bind _ascharacter (Utilities|Casting|CastToCharacter (.HitActor (Collision|BreakHitResult _outhit))))
        (Character|LaunchCharacter _ascharacter (Variables|Default|GetKnockback%20Force) false false)))))

(event Custom|Stop%20Attack
  ;[1 1 1] Cleare Timmer for functions
  (Utilities|Time|ClearandInvalidateTimerbyHandle (Variables|Default|GetTriggerAttack))
  (Utilities|Array|Clear (Variables|Default|GetActors%20to%20Ignore)))

(event Custom|Mele%20trace%20Attack%203d%20for%202%20sockets
  (params (SocketArray :type Array%20of%20Names) (EnemyTagContainer :type Name) (Damage :type Float%20%28double-precision%29) (Attack%20Radius :type Float%20%28double-precision%29) (KnockbackForce :type Vector) (Skeleton%20Mesh :type Skeletal%20Mesh%20Component%20Object%20Reference))
  ;[1 1 1] Melle Attack Calculation for 3D models with exact 2 sockets
  (Variables|Default|SetSocket%20Array SocketArray)
  (Variables|Default|SetEnemy%20Tag%20Container EnemyTagContainer)
  (Variables|Default|SetDamage Damage)
  (Variables|Default|SetAttack%20Radius Attack%20Radius)
  (Variables|Default|SetKnockback%20Force KnockbackForce)
  (Variables|Default|SetSkeleton%20Mesh%20Reference Skeleton%20Mesh)
  (CallFunction|TriggerAttackwith2Sockets))

(event Custom|Trigger%20Attack%20one%20socket
  ;[1 1 1] Mele Attack Calculation for 3D model with one socket attached
  (bind _returnvalue (Utilities|Time|SetTimerbyEvent (delegate Custom|Start%20Attack) 0.01 true))
  (Variables|Default|SetTriggerAttack _returnvalue))

(event Custom|TriggerAttack%20with%202%20sockets
  ;[1 1 1] Melle Attack Calculation for 3D models with exact 2 sockets
  (bind _returnvalue (Utilities|Time|SetTimerbyEvent (delegate Custom|StartAtack2) 0.01 true))
  (Variables|Default|SetTriggerAttack _returnvalue))

(event Custom|Start%20Attack
  (bind _socket_name (Variables|Default|GetSocket%20Name))
  (bind _skeleton_mesh_reference (Variables|Default|GetSkeleton%20Mesh%20Reference))
  (bind _returnvalue (Transformation|GetSocketLocation _skeleton_mesh_reference _socket_name))
  ;[1 1 1] Mele Attack Calculation for 3D model with one socket attached
  (bind _outhit (Collision|SphereTraceByChannel _returnvalue _returnvalue (Variables|Default|GetAttack%20Radius) "TraceTypeQuery2" false (Variables|Default|GetActors%20to%20Ignore) "ForOneFrame"))
  (Utilities|Array|Add (Variables|Default|GetActors%20to%20Ignore) (.HitActor (Collision|BreakHitResult _outhit)))
  (Utilities|IsValid (.HitActor (Collision|BreakHitResult _outhit))
    (:Is%20Valid
      (if (Utilities|Array|ContainsItem (Variables|/Script/Engine.Actor|GetTags (.HitActor (Collision|BreakHitResult _outhit))) (Variables|Default|GetEnemy%20Tag%20Container))
        (Game|Damage|ApplyDamage (.HitActor (Collision|BreakHitResult _outhit)) (Variables|Default|GetDamage) 0 0)
        (bind _ascharacter (Utilities|Casting|CastToCharacter (.HitActor (Collision|BreakHitResult _outhit))))
        (Character|LaunchCharacter _ascharacter (Variables|Default|GetKnockback%20Force) false false)))))

(event EventTick
  (params (DeltaSeconds :type Float%20%28single-precision%29))
  ;[1 1 1] Sphere Trace Calculation 2D
  ;;[0.2568 0.2722 1] If Sprite component is valid we are makeing calculations for 2D character
  (if (Variables|Default|GetIs%20Attaclomg)
    (Utilities|FlowControl|Sequence
      (:then_0
        (Utilities|FlowControl|DoOnce false :!label _label
          (:Completed
            (Variables|Default|SetPrev%20Location (Transformation|GetSocketLocation (Variables|Default|GetSprite) "None"))
            (Utilities|Array|Clear (Variables|Default|GetActors%20to%20Ignore)))))
      (:then_1
        (bind (_array_element _array_index) (Utilities|Array|ForEachLoopwithBreak (Variables|Default|GetSocket%20Array))
          (:LoopBody
            (bind _outhits (Collision|MultiSphereTraceByChannel (Variables|Default|GetPrev%20Location) (Transformation|GetSocketLocation (Variables|Default|GetSprite) _array_element) (Variables|Default|GetAttack%20Radius) "TraceTypeQuery2" false (Variables|Default|GetActors%20to%20Ignore) "ForOneFrame"))
            (Variables|Default|SetPrev%20Location (Transformation|GetSocketLocation (Variables|Default|GetSprite) _array_element))
            (Utilities|FlowControl|Sequence
              (:then_0
                (Utilities|FlowControl|Delay (Variables|Default|GetAttack%20Duration))
                (Variables|Default|SetIs%20Attaclomg false))
              (:then_1
                (for _array_element_2 _outhits
                  (Utilities|Array|Add (Variables|Default|GetActors%20to%20Ignore) (.HitActor (Collision|BreakHitResult _array_element_2)))
                  (if (Utilities|Array|ContainsItem (Variables|/Script/Engine.Actor|GetTags (.HitActor (Collision|BreakHitResult _array_element_2))) (Variables|Default|GetEnemy%20Tag%20Container))
                    (Game|Damage|ApplyDamage (.HitActor (Collision|BreakHitResult _array_element_2)) (Variables|Default|GetDamage) 0 0)
                    (bind _ascharacter (Utilities|Casting|CastToCharacter (.HitActor (Collision|BreakHitResult _array_element_2))))
                    (Character|LaunchCharacter _ascharacter (Variables|Default|GetKnockback%20Force) false false)))))))))
    (else
      (Utilities|Array|Clear (Variables|Default|GetSocket%20Array))
      (goto _label Reset))))