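; Actor component that tracks an owner's health and handles damage, stun and death.
; DamageResponse subtracts damage from Health, triggers Stun, and fires DeathEvent when health reaches zero or below.
; Stun sets IsStuned for StunTime seconds and ignores repeat triggers while active.
; DeathEvent simply destroys the owning actor.
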(event Custom|Stun
  (if (not (Variables|Default|GetIsStuned))
    (Variables|Default|SetIsStuned true)
    (Utilities|FlowControl|Delay (Variables|Default|GetStunTime))
    (Variables|Default|SetIsStuned false)))

(event Custom|DamageResponse
  (params (Damage :type Float%20%28double-precision%29))
  (bind _output_get (Variables|Default|SetDamage Damage))
  (bind _output_get_2 (Variables|Default|SetHealth (- (Variables|Default|GetHealth) _output_get)))
  (CallFunction|Stun)
  (if (<= _output_get_2 0.0)
    (CallFunction|DeathEvent)))

(event Custom|DeathEvent
  (Actor|DestroyActor (Components|GetOwner)))